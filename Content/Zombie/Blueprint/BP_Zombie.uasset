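; BP_Zombie is a zombie enemy that damages the first-person character when its hit box overlaps them.
; On spawn it randomizes mesh scale, yaw and walk speed for variety.
; Kill stops the AI logic, ragdolls the mesh, disables capsule collision, plays a death sound and fires OnKilled after a delay, without destroying the actor.
; A Delay-throttled Tick counts down Timer, usually replaying the death sound.
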(event OnComponentBeginOverlap(hitBox)
  (params (OverlappedComponent :type Primitive%20Component%20Object%20Reference) (OtherActor :type Actor%20Object%20Reference) (OtherComp :type Primitive%20Component%20Object%20Reference) (OtherBodyIndex :type Integer) (bFromSweep :type Boolean) (SweepResult :type Hit%20Result%20Structure%20%28by%20ref%29))
  (bind _asfirst_person_character (Utilities|Casting|CastToFirstPersonCharacter OtherActor))
  (Default|InfligerDegats _asfirst_person_character (Variables|Default|GetPointdeDegats))
  (Audio|PlaySoundatLocation "/Game/Zombie/Ressources/Sons/Zombie_fait_des_degats.Zombie_fait_des_degats" (Transformation|GetActorLocation) "0, 0, 0" 1.0 1.0 0.0 0 0 0))

(event Custom|Kill
  (bind _mesh (Variables|Character|GetMesh))
  (AI|Logic|StopLogic (Variables|/Script/AIModule.AIController|GetBrainComponent (AI|GetAIController self)) "")
  (Collision|SetCollisionProfileName _mesh "Ragdoll" true :!class /Script/Engine.PrimitiveComponent)
  (Physics|SetSimulatePhysics _mesh true)
  (Collision|SetCollisionProfileName (Variables|Collision|GetCapsuleComponent) "NoCollision" true :!class /Script/Engine.PrimitiveComponent)
  (Audio|PlaySoundatLocation "/Game/Zombie/Ressources/Sons/Zombie_meurt.Zombie_meurt" (Transformation|GetActorLocation) "0, 0, 0" 1.0 1.0 0.0 0 0 0)
  (Utilities|FlowControl|Delay 5.0)
  (Default|CallOnKilled self))

(event EventBeginPlay
  (bind _returnvalue (Math|Random|RandomFloatinRange 0.9 1.1))
  (Transformation|SetWorldScale3D (Variables|Character|GetMesh) (Math|Vector|MakeVector _returnvalue _returnvalue _returnvalue))
  (Transformation|SetActorRotation (Math|Rotator|MakeRotator 0.0 0.0 (Math|Random|RandomFloatinRange 0.0 3.6e+02)))
  (Variables|/Script/Engine.CharacterMovementComponent|SetMaxWalkSpeed (Variables|Character|GetCharacterMovement) (Math|Random|RandomFloatinRange 2e+02 4e+02)))

(event EventTick
  (params (DeltaSeconds :type Float%20%28single-precision%29))
  (Utilities|FlowControl|Delay 1.0)
  (if (> (Variables|Default|GetTimer) 0)
    (Variables|Default|SetTimer (- (Variables|Default|GetTimer) 1))
    (if (> 95 (Math|Random|RandomInteger 100))
      (Audio|PlaySoundatLocation "/Game/Zombie/Ressources/Sons/Zombie_meurt.Zombie_meurt" (Transformation|GetActorLocation) "0, 0, 0" 1.0 1.0 0.0 0 0 0))))

(fn ConstructionScript)